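; Player ship for the Galaxian game, handling horizontal movement, firing and hits from enemy fire.
; MoveRight axis input is scaled by MaxSpeed, then consumed on Tick as a frame-rate-independent, swept local offset.
; Fire spawns BP_FriendFire at the Arrow, passes it a player reference and sets FireInProcess to block further shots.
; Box overlap with BP_EnemyFire spawns an explosion, destroys the projectile and notifies GameManager.
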(event OnComponentBeginOverlap(Box)
  (params (OverlappedComponent :type Primitive%20Component%20Object%20Reference) (OtherActor :type Actor%20Object%20Reference) (OtherComp :type Primitive%20Component%20Object%20Reference) (OtherBodyIndex :type Integer) (bFromSweep :type Boolean) (SweepResult :type Hit%20Result%20Structure%20%28by%20ref%29))
  ;[1 1 1] Player hit by Enemy Fire
  (bind _asbp_enemy_fire (Utilities|Casting|CastToBP_EnemyFire OtherActor))
  (Effects|SpawnEmitteratLocation "/Game/Galaxian/StarterContent/Particles/P_Explosion.P_Explosion" (Transformation|GetWorldLocation (Variables|Default|GetBox)))
  (Actor|DestroyActor _asbp_enemy_fire)
  (Default|PlayerHit (Variables|Default|GetGameManager)))

(event EventTick
  (params (DeltaSeconds :type Float%20%28single-precision%29))
  (bind _returnvalue (Class|Pawn|ConsumeMovementInputVector))
  (Transformation|AddActorLocalOffset (* _returnvalue DeltaSeconds) true false))

(event Input|ActionEvents|InputActionFire
  (params (Key :type Key%20Structure :default "None"))
  ;[1 1 1] Generate FriendFire by InputAction (space)
  (:Pressed
    ;;[1 1 1] Fire only once
    (if (not (Variables|Default|GetFireInProcess))
      (bind _returnvalue (Game|SpawnActorfromClass "/Game/Galaxian/Blueprints/BP_FriendFire.BP_FriendFire_C" (Math|Transform|MakeTransform (Transformation|GetWorldLocation (Variables|Default|GetArrow)) "0, 0, 0" "0.700000,0.700000,0.700000") "Undefined" 0 0))
      (Variables|/Game/Galaxian/Blueprints/BP_FriendFire.BP_FriendFire_C|SetPlayer _returnvalue self) ; Keep the Player reference in Fire object
      (Variables|Default|SetFireInProcess true) ; Disable fire twice
    )))

(event Input|AxisEvents|InputAxisMoveRight
  (params (AxisValue :type Float%20%28single-precision%29))
  ;[1 1 1] Move Player left/right with MaxSpeed
  (Pawn|Input|AddMovementInput (Transformation|GetActorRightVector) (* AxisValue (Variables|Default|GetMaxSpeed)) false))

(fn ConstructionScript)