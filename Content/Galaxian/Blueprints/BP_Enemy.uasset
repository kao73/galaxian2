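; BP_Enemy is an enemy actor in a Galaxian game that can shoot and is destroyed when hit by friendly fire.
; A Box overlap with BP_FriendFire spawns an explosion, destroys both actors, notifies the GameManager and refreshes the HUD's enemy display.
; Fire, which has no caller in this Blueprint, spawns a scaled-down BP_EnemyFire at the Arrow and passes it the GameManager reference.
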(event OnComponentBeginOverlap(Box)
  (params (OverlappedComponent :type Primitive%20Component%20Object%20Reference) (OtherActor :type Actor%20Object%20Reference) (OtherComp :type Primitive%20Component%20Object%20Reference) (OtherBodyIndex :type Integer) (bFromSweep :type Boolean) (SweepResult :type Hit%20Result%20Structure%20%28by%20ref%29))
  (bind _gamemanager (Variables|Default|GetGameManager))
  ;[1 1 1] Destroy Enemy when hit by fire
  (bind _asbp_friend_fire (Utilities|Casting|CastToBP_FriendFire OtherActor))
  (Effects|SpawnEmitteratLocation "/Game/Galaxian/StarterContent/Particles/P_Explosion.P_Explosion" (Transformation|GetWorldLocation (Variables|Default|GetBox)))
  (Actor|DestroyActor _asbp_friend_fire)
  (Default|DestroyEnemy _gamemanager self)
  (Actor|DestroyActor)
  (Default|UpdateEnemies (Variables|/Game/Galaxian/Blueprints/BP_GameManager.BP_GameManager_C|GetHUDWidget _gamemanager)))

(fn ConstructionScript)

(fn Fire
  (bind _returnvalue (Game|SpawnActorfromClass "/Game/Galaxian/Blueprints/BP_EnemyFire.BP_EnemyFire_C" (Math|Transform|MakeTransform (Transformation|GetWorldLocation (Variables|Default|GetArrow)) "0,0.000000,180.000000" "0.700000,0.700000,0.700000") "Undefined" 0 0))
  (Variables|/Game/Galaxian/Blueprints/BP_EnemyFire.BP_EnemyFire_C|SetGameManager _returnvalue (Variables|Default|GetGameManager)))